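; Game manager for an elevator game that shows the main menu in a widget component and runs the session between StartGame and EndGame.
; A delay-driven loop rides between floors with motor sounds and camera shakes, bumps the level display, opens the doors and spawns a random class at a random spawn point before closing them.
; EndGame restores the menu, destroys all spawned actors, stops the music and resets the display.
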(event Custom|StartElevator
  ;[1 1 1] Start Elevator
  (Audio|PlaySoundatLocation "/Game/PersonalSpaceInvader/Audio/A_ElevatorMotorStart.A_ElevatorMotorStart" "0, 0,250.000000")
  (Camera|PlayWorldCameraShake "/Game/PersonalSpaceInvader/Blueprints/BP_ElevatorSTartShake.BP_ElevatorStartShake_C" "0, 0,-20.000000" 0.0 1e+03)
  (Utilities|FlowControl|Delay 1.0)
  (bind _returnvalue (Audio|SpawnSoundatLocation "/Game/PersonalSpaceInvader/Audio/A_ElevatorMotorRunningLoop.A_ElevatorMotorRunningLoop" "0, 0,250.000000"))
  (Variables|Default|SetAudioElevatorLoopComponent _returnvalue))

(event Custom|StartGame
  (bind _widget (Variables|Default|GetWidget))
  (bind _spawnclasses (Variables|Default|GetSpawnClasses))
  (bind _spawnpoints (Variables|Default|GetSpawnPoints))
  ;[1 1 1] Gameplay management
  (Rendering|SetVisibility _widget false false)
  (Components|Activation|SetActive _widget false false)
  (Variables|Default|SetGameActive true)
  (bind _returnvalue (Audio|SpawnSoundatLocation "/Game/PersonalSpaceInvader/Audio/A_ElevatorMusicRecut.A_ElevatorMusicRecut" "0.000000, 0,260.000000" "0, 0, 0" 0.6 1.0 0.0))
  (Variables|Default|SetMusic _returnvalue)
  (Utilities|FlowControl|Sequence
    (:then_0
      (Audio|Components|Audio|FadeIn (Variables|Default|GetMusic) 3.0 0.6 0.0 :!class /Script/Engine.AudioComponent))
    (:then_1
      (CallFunction|StartElevator :!label _label)
      (Utilities|FlowControl|Delay (Variables|Default|GetLevelTime))
      (CallFunction|StopElevator)
      (Utilities|FlowControl|Delay 1.0)
      (Default|IncreaseLevel (Variables|Default|GetLevelDisplay))
      (Utilities|FlowControl|Delay 0.4)
      (Default|DoorTrigger (Variables|Default|GetDoors) true)
      (if (Variables|Default|GetGameActive)
        (Game|SpawnActorfromClass (Utilities|Array|Get(acopy) _spawnclasses (Math|Random|RandomInteger (Utilities|Array|Length _spawnclasses))) (Transformation|GetActorTransform (Utilities|Array|Get(acopy) _spawnpoints (Math|Random|RandomInteger (Utilities|Array|Length _spawnpoints)))) "Undefined" 0 0)
        (Utilities|FlowControl|Delay (Variables|Default|GetLoadTime))
        (Default|DoorTrigger (Variables|Default|GetDoors) false)
        (Utilities|FlowControl|Delay 4.8)
        (if (Variables|Default|GetGameActive)
          (goto _label))))))

(event Custom|EndGame
  (bind _leveldisplay (Variables|Default|GetLevelDisplay))
  (bind _widget (Variables|Default|GetWidget))
  ;[1 1 1] End game
  (if (Variables|Default|GetGameActive)
    (Variables|Default|SetGameActive false)
    (Rendering|SetVisibility _widget true false)
    (Components|Activation|SetActive _widget true false)
    (for _array_element (Variables|Default|GetSpawnClasses)
      (bind _outactors (Actor|GetAllActorsOfClass _array_element))
      (for _array_element_2 _outactors
        (Actor|DestroyActor _array_element_2)))
    (Audio|Components|Audio|Stop (Variables|Default|GetMusic))
    (Variables|/Game/PersonalSpaceInvader/Blueprints/BP_ElevatorDisplay.BP_ElevatorDisplay_C|SetLevel _leveldisplay 0)
    (Rendering|Components|TextRender|SetText (Variables|/Game/PersonalSpaceInvader/Blueprints/BP_ElevatorDisplay.BP_ElevatorDisplay_C|GetTextRender _leveldisplay) (Utilities|Text|ToText(String) "E"))))

(event Custom|StopElevator
  ;[1 1 1] Stop Elevator
  (Audio|Components|Audio|Stop (Variables|Default|GetAudioElevatorLoopComponent))
  (Audio|PlaySoundatLocation "/Game/PersonalSpaceInvader/Audio/A_ElevatorMotorStop.A_ElevatorMotorStop" "0, 0,250.000000")
  (Camera|PlayWorldCameraShake "/Game/PersonalSpaceInvader/Blueprints/BP_ElevatorStopShake.BP_ElevatorStopShake_C" "0, 0,-20.000000" 0.0 1e+03))

(event EventBeginPlay
  (bind _returnvalue (Game|GetPlayerController 0))
  (bind _returnvalue_2 (UserInterface|CreateWidget "/Game/PersonalSpaceInvader/UI/MainMenu.MainMenu_C" _returnvalue))
  (bind _output_get (Variables|Default|SetMenu _returnvalue_2))
  (UserInterface|SetWidget (Variables|Default|GetWidget) _output_get)
  (Input|EnableInput _returnvalue))

(fn ConstructionScript)