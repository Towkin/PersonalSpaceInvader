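; Behavior Tree task that picks a random elevator spot for a passenger and writes its location to the blackboard.
; It gathers all BP_ElevatorSpot actors, shuffles them, stores the first one's location in SpotKey and finishes with success.
; A sphere overlap check for passengers already at the spot is present but disconnected, so occupied spots can be chosen.
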(event EventReceiveExecute
  (params (OwnerActor :type Actor%20Object%20Reference))
  (bind _outactors (Actor|GetAllActorsOfClass "/Game/PersonalSpaceInvader/Blueprints/BP_ElevatorSpot.BP_ElevatorSpot_C"))
  (Utilities|Array|Shuffle _outactors)
  (bind _array_element (Utilities|Array|ForEachLoopwithBreak _outactors :!label _label)
    (:LoopBody
      (AI|BehaviorTree|SetBlackboardValueasVector (Variables|Default|GetSpotKey) (Transformation|GetActorLocation _array_element))
      (goto _label Break))
    (:Completed
      (AI|BehaviorTree|FinishExecute true))))