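; Elevator display actor for PersonalSpaceInvader that shows the current level number on a text render component.
; Its IncreaseLevel event increments the Level counter, writes the value to the text and conditionally plays a ding sound at the actor's location.
; The construction script is empty, and the file contains no trigger for the event, only the event itself.
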(event Custom|IncreaseLevel
  (bind _result (Math|Integer|IncrementInt (Variables|Default|GetLevel))
    (:%20%20
      (Rendering|Components|TextRender|SetText (Variables|Default|GetTextRender) (Utilities|Text|ToText(Integer) _result))
      (if (!= (Variables|Default|GetElevatorDingAudio) 0)
        (Audio|PlaySoundatLocation (Variables|Default|GetElevatorDingAudio) (Transformation|GetActorLocation))))))

(fn ConstructionScript)