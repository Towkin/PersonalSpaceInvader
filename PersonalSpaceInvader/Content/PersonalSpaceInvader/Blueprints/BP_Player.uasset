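; VR player for Personal Space Invader that builds up anxiety while other pawns intrude on the space around the headset.
; Each tick, a debug-drawn sphere overlap at the HMD position raises or lowers a clamped anxiety timer.
; The squared anxiety percentage scales down a camera post-process vector, and full anxiety calls EndGame on BP_Manager.
; Intermediate anxiety threshold checks trigger nothing.
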(event EventBeginPlay
  (|CallParentFunction))

(event EventTick
  (params (DeltaSeconds :type Float%20%28single-precision%29))
  (bind (_devicerotation _deviceposition) (Class|HeadMountedDisplayFunctionLibrary|GetOrientationandPosition))
  (bind _percentage (Utilities|AnxietyPercent))
  (bind _returnvalue (* _percentage _percentage))
  (bind _returnvalue_2 (- 1.0 _returnvalue))
  (|CallParentFunction DeltaSeconds)
  (bind _output_get (Variables|Default|SetHeadTransform (Math|Transform|ComposeTransforms (Math|Transform|MakeTransform _deviceposition _devicerotation) (Transformation|GetRelativeTransform (Variables|Default|GetVROrigin)))))
  (bind _returnvalue_3 (Class|KismetSystemLibrary|SphereOverlapActorsNEW (.Location (Math|Transform|BreakTransform _output_get)) 45.0 (Utilities|Array|MakeArray "ObjectTypeQuery3") 0 (Utilities|Array|MakeArray self)))
  (Rendering|Debug|DrawDebugSphere (.Location (Math|Transform|BreakTransform _output_get)) 45.0 12 "(R=1.000000,G=0.000000,B=0.000000,A=1.000000)" DeltaSeconds 5.0)
  (Variables|Default|SetAnxietyTimer (Math|Float|Clamp(Float) (+ (Variables|Default|GetAnxietyTimer) (* DeltaSeconds (select _returnvalue_3 1.0 -1.0))) 0.0 (Variables|Default|GetAnxietyTimerMax)))
  (Utilities|FlowControl|Sequence
    (:then_0
      (Variables|/Script/Engine.CameraComponent|SetPostProcessSettings (Variables|Default|GetCamera) (Utilities|Struct|MakePostProcessSettings (Math|Vector4|MakeVector4 _returnvalue_2 _returnvalue_2 _returnvalue_2 _returnvalue_2))))
    (:then_1
      (if (== _percentage 1.0)
        (bind _outactors (Actor|GetAllActorsOfClass "/Game/PersonalSpaceInvader/Blueprints/BP_Manager.BP_Manager_C"))
        (Default|EndGame (Utilities|Array|Get(acopy) _outactors))
        (elif (not (> _percentage 0.8))
          (if (not (> _percentage 0.5))
            (if (> _percentage 0.2)
              _)))))))

(fn ConstructionScript
  (|CallParentFunction))