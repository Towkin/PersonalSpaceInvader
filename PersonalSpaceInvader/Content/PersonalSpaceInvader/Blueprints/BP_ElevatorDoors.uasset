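; Elevator doors Blueprint that slides a left and right door panel open or closed.
; The DoorTrigger event takes an Open flag, playing the matching optional sound at the actor's location and running a timeline forward or in reverse.
; The timeline's alpha lerps both panels' relative Y offsets in opposite directions between closed and open positions.
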(event Custom|DoorTrigger
  (params (Open :type Boolean))
  (bind _dooropensound (Variables|Default|GetDoorOpenSound))
  (bind _doorclosesound (Variables|Default|GetDoorCloseSound))
  (if Open
    (if (!= _dooropensound 0)
      (Audio|PlaySoundatLocation _dooropensound (Transformation|GetActorLocation))
      (bind _alpha (Timeline|DoorTimeline Play)
        (:Update
          (Transformation|SetRelativeLocation (Variables|Default|GetLeftDoor) (Math|Vector|Lerp(Vector) "0,-45.500000, 0" "0,-120.000000, 0" _alpha) false false)
          (Transformation|SetRelativeLocation (Variables|Default|GetRightDoor) (Math|Vector|Lerp(Vector) "0,45.500000, 0" "0,120.000000, 0" _alpha) false false)))
      (else
        (Timeline|DoorTimeline Play)))
    (elif (!= _doorclosesound 0)
      (Audio|PlaySoundatLocation _doorclosesound (Transformation|GetActorLocation))
      (Timeline|DoorTimeline Reverse)
      (else
        (Timeline|DoorTimeline Reverse)))))

(fn ConstructionScript)